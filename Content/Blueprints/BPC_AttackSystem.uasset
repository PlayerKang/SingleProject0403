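; Actor component that gives the third-person character a four-step melee combo of sword swings and a kick.
; Attack input, gated by CanAttack, plays the montage for the current AttackIndex or buffers the press if already attacking.
; SwordAttackCombo consumes a buffered press to chain the next step, otherwise resets the combo.
; Input also starts a looping sphere trace along the sword that draws debug shapes; hits are unused and the timer is never cleared.
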(event `self.ReceiveBeginPlay`
  (bind _asbp_third_person_character (cast `/Game/ThirdPerson/Blueprints/BP_ThirdPersonCharacter` (`self.GetOwner`)))
  (set `self.Character BP` _asbp_third_person_character)
  (set `self.Character Mesh` (`Character.Mesh` _asbp_third_person_character)))

(event `Attack 1`
  ;[1 0.2124 0.1427] Combo
  ;;[1 1 1] Attack 1
  (`/Engine/EditorBlueprintResources/StandardMacros.DoOnce` false :!label _label
    (:`Completed`
      (`KismetSystemLibrary.Delay` 0.1)
      (`|PlayMontage` (`self.Character Mesh`) "/Game/Animation/Combat/SwordAttack/Attack1_Montage.Attack1_Montage"
        (:`then`
          (set `self.Attack Index` 1)
          (goto _label :!via `Reset`))))))

(event `EnhancedInput|/Game/Input/IA_Attack`
  (params (ActionValue :type Boolean) (ElapsedSeconds :type "Float (double-precision)") (TriggeredSeconds :type "Float (double-precision)") (InputAction :type "InputAction Object Reference" :default "/Game/Input/IA_Attack.IA_Attack"))
  ;[1 0.2124 0.1427] Combo
  ;;[1 1 1] Attack Input
  (:`Started`
    (if (`self.canAttack?`)
      (`self.Sword Attack`)
      (`self.Start Sword Trace`))))

(event `Attack 2`
  ;[1 0.2124 0.1427] Combo
  ;;[1 1 1] Attack 2
  (`/Engine/EditorBlueprintResources/StandardMacros.DoOnce` false :!label _label_2
    (:`Completed`
      (`KismetSystemLibrary.Delay` 0.1)
      (`|PlayMontage` (`self.Character Mesh`) "/Game/Animation/Combat/SwordAttack/Attack2_Montage.Attack2_Montage"
        (:`then`
          (set `self.Attack Index` 2)
          (goto _label_2 :!via `Reset`))))))

(event `Sword Attack`
  ;[1 0.2124 0.1427] Combo
  ;;[1 1 1] Sword Attack
  (if (`self.isAttacking?`)
    (set `self.saveAttack?` true)
    (else
      (set `self.isAttacking?` true)
      (switch `int` (`self.Attack Index`) :!label _label_3
        (:`0`
          (`self.Attack 1`))
        (:`1`
          (`self.Attack 2`))
        (:`2`
          (`self.Attack 3`))
        (:`3`
          (`self.Attack4`))))))

(event `Attack 3`
  ;[1 0.2124 0.1427] Combo
  ;;[1 1 1] Attack 3
  (`/Engine/EditorBlueprintResources/StandardMacros.DoOnce` false :!label _label_4
    (:`Completed`
      (`KismetSystemLibrary.Delay` 0.1)
      (`|PlayMontage` (`self.Character Mesh`) "/Game/Animation/Combat/SwordAttack/Kick_Montage.Kick_Montage"
        (:`then`
          (set `self.Attack Index` 3)
          (goto _label_4 :!via `Reset`))))))

(event `SwordAttackCombo`
  ;[1 0.2124 0.1427] Combo
  ;;[1 1 1] Combo Continue
  (if (`self.saveAttack?`)
    (set `self.saveAttack?` false)
    (goto _label_3)
    (else
      (`self.Stop Combo`))))

(event `Attack4`
  ;[1 0.2124 0.1427] Combo
  ;;[1 1 1] Attack4
  (`/Engine/EditorBlueprintResources/StandardMacros.DoOnce` false :!label _label_5
    (:`Completed`
      (`KismetSystemLibrary.Delay` 0.1)
      (`|PlayMontage` (`self.Character Mesh`) "/Game/Animation/Combat/SwordAttack/Attack3_Montage.Attack3_Montage"
        (:`then`
          (set `self.Attack Index` 4)
          (goto _label_5 :!via `Reset`))))))

(event `Stop Combo`
  ;[1 0.2124 0.1427] Combo
  ;;[1 1 1] Stop Combo / Attack
  (set `self.isAttacking?` false)
  (set `self.Attack Index` 0))

(event `Start Sword Trace`
  (`KismetSystemLibrary.K2_SetTimerDelegate` (delegate `Sword Trace Loop`) 0.1 true))

(event `Sword Trace Loop`
  (bind _character_bp (`self.Character BP`))
  (`KismetSystemLibrary.SphereTraceSingle` :`Start` (`SceneComponent.K2_GetComponentLocation` (`/Game/ThirdPerson/Blueprints/BP_ThirdPersonCharacter.Sword Top` _character_bp)) :`End` (`SceneComponent.K2_GetComponentLocation` (`/Game/ThirdPerson/Blueprints/BP_ThirdPersonCharacter.Sword Bottom` _character_bp)) :`Radius` 5.0 :`TraceChannel` "TraceTypeQuery1" :`DrawDebugType` "ForDuration" :`DrawTime` 0.1))