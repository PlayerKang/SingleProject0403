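; BP_Pocket is a container for a list of balls that can be added to, shuffled and drawn from.
; BeginPlay calls Push 45 times with no ball supplied, and Push appends its input before a BP_Ball cast that leads nowhere.
; Shuffle randomizes the list order.
; Draw removes the entry at index zero, then returns index zero of the list.
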(event `self.ReceiveBeginPlay`
  (for _ (range 45)
    (`self.Push` null)))

(fn `Draw`
  (returns (DrawBall :type "/Game/Blueprints/BP_Ball Object Reference"))
  (bind _balls (`self.Balls`))
  (bind _output (`|GetArrayItem` _balls))
  (`KismetArrayLibrary.Array_RemoveItem` _balls _output)
  (return _output))

(fn `Push`
  (params (Balls :type "/Game/Blueprints/BP_Ball Object Reference"))
  (`KismetArrayLibrary.Array_Add` (`self.Balls`) Balls)
  (cast `/Game/Blueprints/BP_Ball` Balls))

(fn `Shuffle`
  (`KismetArrayLibrary.Array_Shuffle` (`self.Balls`)))

(fn `UserConstructionScript`)